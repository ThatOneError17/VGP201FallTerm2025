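; BP_Door is a door actor that removes itself from the level once all of its targets are destroyed.
; BeginPlay sets a remaining-target counter from the length of the Targets array.
; Each TargetDestroyed call decrements the counter, and the door destroys itself at zero.
; The door does not bind to its targets here, and an unconnected validity-check loop over Targets never runs.
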(event `self.ReceiveBeginPlay`
  (set `self.RemainingTargets` (`KismetArrayLibrary.Array_Length` (`self.Targets`))))

(event `TargetDestroyed`
  (bind _output_get (set `self.RemainingTargets` (- (`self.RemainingTargets`) 1)))
  (if (== _output_get 0)
    (`self.K2_DestroyActor`)))

(fn `UserConstructionScript`)