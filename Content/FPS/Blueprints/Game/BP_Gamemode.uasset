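; BP_Gamemode is the FPS game mode that tracks a timer and score and manages the game menu and game-over screens.
; BeginPlay spawns WBP_GameMenu with game-only input, then pushes GameTimer and Score to it.
; Tick drives IncreaseTimer, whose one-second Delay paces the count and menu refresh.
; GameOver shows WBP_GameOverMenu with UI-only input and the cursor; an unconnected example spawns the player's starting rifle.
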(event `self.ReceiveBeginPlay`
  (`KismetSystemLibrary.PrintString` "Spawning BP_Gamemode")
  (`self.SpawnGameMenu`)
  (`self.UpdateTimer`)
  (`self.UpdateScore`))

(event `self.ReceiveTick`
  (params (DeltaSeconds :type "Float (single-precision)"))
  (`self.IncreaseTimer`))

(event `GameOver`
  (bind _returnvalue (`GameplayStatics.GetPlayerController` 0))
  (bind _returnvalue_2 (`|CreateWidget` "/Game/FPS/Blueprints/Game/GUI/WBP_GameOverMenu.WBP_GameOverMenu_C"))
  (bind _output_get (set `self.GameOverRef` _returnvalue_2))
  (`UserWidget.AddToViewport` _output_get 0)
  (`WidgetBlueprintLibrary.SetInputMode_UIOnlyEx` _returnvalue (`self.GameOverRef`))
  (set `PlayerController.bShowMouseCursor` true _returnvalue))

(fn `SpawnGameMenu`
  (bind _returnvalue (`GameplayStatics.GetPlayerController` 0))
  (bind _returnvalue_2 (`|CreateWidget` "/Game/FPS/Blueprints/Game/GUI/WBP_GameMenu.WBP_GameMenu_C"))
  (bind _output_get (set `self.MenuRef` _returnvalue_2))
  (`UserWidget.AddToViewport` _output_get 0)
  (`WidgetBlueprintLibrary.SetInputMode_GameOnly` _returnvalue)
  (set `PlayerController.bShowMouseCursor` false _returnvalue))

(fn `UpdateScore`
  (bind _aswbp_game_menu (cast `/Game/FPS/Blueprints/Game/GUI/WBP_GameMenu` (`self.MenuRef`)))
  (`/Game/FPS/Blueprints/Game/GUI/WBP_GameMenu.UpdateScore` _aswbp_game_menu (`self.Score`)))

(fn `UpdateTimer`
  (bind _aswbp_game_menu (cast `/Game/FPS/Blueprints/Game/GUI/WBP_GameMenu` (`self.MenuRef`)))
  (`/Game/FPS/Blueprints/Game/GUI/WBP_GameMenu.UpdateTimer` _aswbp_game_menu (`self.GameTimer`)))

(fn `UserConstructionScript`)