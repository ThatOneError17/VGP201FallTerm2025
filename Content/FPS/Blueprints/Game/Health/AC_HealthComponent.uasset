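; Actor component that tracks an owner's health in the FPS game, starting at maximum on BeginPlay.
; Damage and Heal accept only positive amounts, printing a warning otherwise, and route through SetHealth, which clamps between minimum and maximum.
; Helpers provide a full heal, a normalized 0–1 health value and an IsDead check against the minimum.
; It has no event dispatchers, so health and death state are read by querying it.
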(event `self.ReceiveBeginPlay`
  (bind _maxhealth (`self.MaxHealth`))
  (`self.Init` (`self.MinHealth`) _maxhealth _maxhealth))

(fn `ClampHealth`
  (params (Value :type "Float (double-precision)"))
  (returns (ReturnValue :type "Float (double-precision)"))
  (return (`KismetMathLibrary.FClamp` Value (`self.MinHealth`) (`self.MaxHealth`))))

(fn `Damage`
  (params (DamageAmount :type "Float (double-precision)"))
  (if (> DamageAmount 0.0)
    (`self.SetHealth` (- (`self.GetHealth`) DamageAmount))
    (else
      (`KismetSystemLibrary.PrintString` "Damage Amount must be positive"))))

(fn `GetHealth`
  (returns (Health :type "Float (double-precision)"))
  (return (`self.Health`)))

(fn `GetNormalizeHealth`
  (returns (NormalizeHealth :type "Float (double-precision)"))
  (return (`KismetMathLibrary.FClamp` (/ (`self.GetHealth`) (`self.MaxHealth`)))))

(fn `Heal`
  (params (GainHealth :type "Float (double-precision)"))
  (if (> GainHealth 0.0)
    (`self.SetHealth` (+ (`self.GetHealth`) GainHealth))
    (else
      (`KismetSystemLibrary.PrintString` "Heal amount must be positive"))))

(fn `HealFull`
  (`self.Heal` (`self.MaxHealth`)))

(fn `Init`
  (params (MinHealth :type "Float (double-precision)") (MaxHealth :type "Float (double-precision)") (NewHealth :type "Float (double-precision)"))
  (set `self.MinHealth` MinHealth)
  (set `self.MaxHealth` MaxHealth)
  (`self.SetHealth` NewHealth))

(fn `IsDead`
  (returns (Value :type Boolean))
  (return (<= (`self.GetHealth`) (`self.MinHealth`))))

(fn `SetHealth`
  (params (NewHealth :type "Float (double-precision)"))
  (returns (Health :type "Float (double-precision)"))
  (bind _output_get (set `self.Health` (`self.ClampHealth` NewHealth)))
  (return _output_get))