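; BP_EnemyAICharacter is an enemy AI character that takes damage and awards score to the game mode when killed.
; AnyDamage passes damage to its health component, then checks whether the enemy is dead.
; On death it destroys itself and sends its Score to BP_Gamemode's UpdateScore; otherwise it prints the remaining health.
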(event `self.ReceiveAnyDamage`
  (params (Damage :type "Float (single-precision)") (DamageType :type "DamageType Object Reference") (InstigatedBy :type "Controller Object Reference") (DamageCauser :type "Actor Object Reference"))
  (bind _ac_healthcomponent (`self.AC_HealthComponent`))
  (`/Game/FPS/Blueprints/Game/Health/AC_HealthComponent.Damage` _ac_healthcomponent Damage)
  (if (`/Game/FPS/Blueprints/Game/Health/AC_HealthComponent.IsDead` _ac_healthcomponent)
    (`self.K2_DestroyActor`)
    (bind _asbp_gamemode (cast `/Game/FPS/Blueprints/Game/BP_Gamemode` (`GameplayStatics.GetGameMode`)))
    (`/Game/FPS/Blueprints/Game/BP_Gamemode.UpdateScore` _asbp_gamemode (`self.Score`))
    (else
      (`KismetSystemLibrary.PrintString` (`KismetStringLibrary.Conv_DoubleToString` (`/Game/FPS/Blueprints/Game/Health/AC_HealthComponent.GetHealth` _ac_healthcomponent))))))

(fn `UserConstructionScript`)